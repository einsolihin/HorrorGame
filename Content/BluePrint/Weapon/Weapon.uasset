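; Weapon actor attached to a BaseCharacter that handles hitscan firing, ammo and reloading.
; FireEvent fires once for "Gun" types or sets trigger flags while aiming, letting Tick repeat camera line traces passed to the character's Hit.
; FireAgain adds crosshair feedback, recoil and a fire-rate delay.
; Tick prints ammo for debugging and calls reload on an empty magazine through an authority switch, alongside replicated state with empty OnReps.
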(event Custom|PrintBullet
  (Development|PrintString (Utilities|String|ToString(Text) (Utilities|Text|FormatText "Bullet = {Bullet}  
Ammo = {Ammo}" (Utilities|Text|ToText(Integer) (Variables|Ammo|GetBullet)) (Utilities|Text|ToText(Integer) (Variables|Ammo|GetCurrentAmmo)))) true true "(R=0.000000,G=0.660000,B=1.000000,A=1.000000)" (Variables|Default|GetDeltaTime)))

(event Custom|WeaponReload
  ;[1 1 1] Reloading
  (if (== (Variables|Ammo|GetBullet) (Variables|Ammo|GetAmmo))
    (Variables|Fire|SetisReload true)
    (if (> (Variables|Ammo|GetCurrentAmmo) 0)
      (if (<= (- (Variables|Ammo|GetCurrentAmmo) (- (Variables|Ammo|GetAmmo) (Variables|Ammo|GetBullet))) 0)
        (Variables|Ammo|SetBullet (- (- (Variables|Ammo|GetAmmo) (Variables|Ammo|GetBullet)) (Variables|Ammo|GetCurrentAmmo)))
        (Variables|Ammo|SetCurrentAmmo 0)
        (else
          (Variables|Ammo|SetCurrentAmmo (- (Variables|Ammo|GetCurrentAmmo) (- (Variables|Ammo|GetAmmo) (Variables|Ammo|GetBullet))))
          (Variables|Ammo|SetBullet (Variables|Ammo|GetAmmo))))
      (Utilities|FlowControl|Delay 2.0)
      (Variables|Fire|SetisReload false))))

(event Custom|Call%20Set%20Ammo
  (CallFunction|SetAmmo))

(event Custom|Set%20Ammo
  (bind _asbase_character (Utilities|Casting|CastToBaseCharacter (Actor|GetParentActor)))
  (Variables|/Game/BluePrint/Character/BaseCharacter.BaseCharacter_C|SetCurrentAmmo _asbase_character (Variables|Ammo|GetCurrentAmmo))
  (Variables|/Game/BluePrint/Character/BaseCharacter.BaseCharacter_C|SetBullet _asbase_character (Variables|Ammo|GetBullet)))

(event Custom|FireLineTrace
  ;[1 1 1] Fire a LineTrace
  (bind _asbase_character (Utilities|Casting|CastToBaseCharacter (Actor|GetParentActor)))
  (CallFunction|BulletDeduction)
  (bind _outhit (Collision|LineTraceByChannel (Transformation|GetWorldLocation (Variables|/Game/BluePrint/Character/BaseCharacter.BaseCharacter_C|GetCamera _asbase_character)) (+ (Transformation|GetWorldLocation (Variables|/Game/BluePrint/Character/BaseCharacter.BaseCharacter_C|GetCamera _asbase_character)) (* (Math|Vector|GetForwardVector (Variables|/Game/BluePrint/Character/BaseCharacter.BaseCharacter_C|GetCamera _asbase_character)) 1e+03)) "TraceTypeQuery1" false 0 "ForDuration"))
  (|FireAgain)
  (bind _asbase_character_2 (Utilities|Casting|CastToBaseCharacter (Actor|GetParentActor)))
  (Default|Hit _asbase_character_2 _outhit))

(event Custom|Call%20Fire%20Line%20Trace
  ;[1 1 1] Event Tick
  (CallFunction|FireLineTrace))

(event Custom|FireEvent
  (params (isFire :type Boolean))
  ;[1 1 1] Fire
  (if (Utilities|Enum|Equal(Enum) (Variables|Fire|GetWeaponType) "Gun")
    (CallFunction|FireLineTrace)
    (elif (Variables|Fire|GetisAim?)
      (Variables|Fire|SetisFire? isFire)
      (Variables|Fire|SetisTrigger? isFire))))

(event Custom|Call%20Reload
  ;[1 1 1] Event Tick
  (CallFunction|WeaponReload))

(event Custom|CallFire
  ;[1 1 1] Fire
  (CallFunction|CallFireLineTrace))

(event Custom|Bullet%20Deduction
  (bind _result (Math|Integer|DecrementInt (Variables|Ammo|GetBullet))
    (:%20%20
      (Variables|Ammo|SetBullet _result))))

(event EventBeginPlay
  ;[1 1 1] Start Game
  (Variables|Ammo|SetBullet (Variables|Ammo|GetAmmo))
  (Variables|Ammo|SetCurrentAmmo (Variables|Ammo|GetMaxAmmo))
  (if (Utilities|Enum|Equal(Enum) (Variables|Fire|GetWeaponType) "Semi Auto")
    (Variables|Fire|SetCurrentFire (Variables|Fire|GetFireBurst))))

(event EventTick
  (params (DeltaSeconds :type Float%20%28single-precision%29))
  ;[1 1 1] Event Tick
  (Variables|Default|SetDeltaTime DeltaSeconds)
  (CallFunction|PrintBullet)
  (if (<= (Variables|Ammo|GetBullet) 0)
    (Variables|Fire|SetisFire? false)
    (Networking|SwitchHasAuthority
      (:Authority
        (CallFunction|WeaponReload))
      (:Remote
        (CallFunction|CallReload)))
    (elif (Math|Boolean|ANDBoolean (Variables|Fire|GetisAim?) (Variables|Fire|GetisFire?) (> (Variables|Ammo|GetBullet) 0) (not (Variables|Fire|GetisReload)) (Variables|Fire|GetisTrigger?))
      (CallFunction|FireLineTrace)
      (else
        (Variables|Fire|SetisFire? false)))))

(fn ConstructionScript)

(fn OnRepIsFire?)

(fn OnRepIsAim?)

(fn OnRepIsReload)

(fn OnRepIsTrigger?)

(fn OnRepBullet)