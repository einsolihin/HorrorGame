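; Game instance that manages front-end menus, multiplayer sessions and network error reporting.
; A save-slot check opens either the main menu or, without a save, the options menu with a welcome message.
; Hosting and joining show a loading screen, with successful hosting opening the Lobby level.
; Most widgets are cached for reuse, while session, network and travel failures feed a shared error dialog, with most network failures reported as lost host connection.
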(event Custom|ShowMainMenu
  (bind _returnvalue (Game|GetPlayerController 0))
  ;[1 1 1] Show Main Menu
  (Utilities|IsValid (Variables|Widget|GetMainMenuWB)
    (:Is%20Valid
      _)
    (:Is%20Not%20Valid
      (bind _returnvalue_2 (UserInterface|CreateWidget "/Game/UI/MainMenu/MainMenu.MainMenu_C" _returnvalue))
      (Variables|Widget|SetMainMenuWB _returnvalue_2)))
  (UserInterface|Viewport|AddtoViewport (Variables|Widget|GetMainMenuWB) 0)
  (Variables|/Script/Engine.PlayerController|SetbShowMouseCursor _returnvalue true))

(event Custom|Show%20Host%20Menu
  ;[1 1 1] Host Game Menu
  (Utilities|IsValid (Variables|Widget|GetHostMenuWB)
    (:Is%20Valid
      _)
    (:Is%20Not%20Valid
      (bind _returnvalue (UserInterface|CreateWidget "/Game/UI/MainMenu/HostMenu.HostMenu_C" (Game|GetPlayerController 0)))
      (Variables|Widget|SetHostMenuWB _returnvalue)))
  (UserInterface|Viewport|AddtoViewport (Variables|Widget|GetHostMenuWB) 0))

(event Custom|Show%20Server%20Menu
  ;[1 1 1] Shows the Server Menu
  (bind _returnvalue (UserInterface|CreateWidget "/Game/UI/MainMenu/ServerMenu.ServerMenu_C" (Game|GetPlayerController 0)))
  (UserInterface|Viewport|AddtoViewport _returnvalue 0))

(event Custom|Show%20Option%20Menu
  ;[1 1 1] Show the Option Menu
  (Utilities|IsValid (Variables|Widget|GetOptionMenuWB)
    (:Is%20Valid
      _)
    (:Is%20Not%20Valid
      (bind _returnvalue (UserInterface|CreateWidget "/Game/UI/MainMenu/OptionMenu.OptionMenu_C" (Game|GetPlayerController 0)))
      (Variables|Widget|SetOptionMenuWB _returnvalue)))
  (UserInterface|Viewport|AddtoViewport (Variables|Widget|GetOptionMenuWB) 0)
  (if (not (Variables|Default|GetCreatedSaveFile?))
    (Variables|/Game/UI/MainMenu/OptionMenu.OptionMenu_C|SetWelcomeMessageVis (Variables|Widget|GetOptionMenuWB) "Visible")))

(event Custom|LaunchLobby
  (params (NumberOfPlayer :type Integer) (EnableLan :type Boolean) (ServerName :type Text))
  ;[1 1 1] Launch Lobby
  (Variables|ServerSettings|SetMaxPlayer NumberOfPlayer)
  (Variables|ServerSettings|SetServer%20Name ServerName)
  (CallFunction|ShowLoadingScreen)
  (|Session (Game|GetPlayerController 0) (Variables|ServerSettings|GetMaxPlayer) EnableLan
    (:OnSuccess
      (Game|OpenLevel(byName) "Lobby" true "listen"))
    (:OnFailure
      (Utilities|DisplayErrorMessage "Failed to create seesion. Please Try Again."))))

(event Custom|ShowLoadingScreen
  ;[1 1 1] Show Loading Screen
  (Utilities|IsValid (Variables|Widget|GetLoadingScreenWB)
    (:Is%20Valid
      _)
    (:Is%20Not%20Valid
      (bind _returnvalue (UserInterface|CreateWidget "/Game/UI/AllLevel/LoadingScreen.LoadingScreen_C" (Game|GetPlayerController 0)))
      (Variables|Widget|SetLoadingScreenWB _returnvalue)))
  (UserInterface|Viewport|AddtoViewport (Variables|Widget|GetLoadingScreenWB) 0))

(event Custom|Join%20Server
  (params (Session%20to%20join :type Blueprint%20Session%20Result%20Structure))
  ;[1 1 1] Join Server
  (CallFunction|ShowLoadingScreen)
  (|JoinSession (Game|GetPlayerController 0) Session%20to%20join
    (:OnFailure
      (Utilities|DisplayErrorMessage "Fail to join Session. Please Try Again"))))

(event Custom|Destroy%20Seesion%20Caller
  (params (PlayerController :type Player%20Controller%20Object%20Reference))
  ;[1 1 1] Destroy Session When Called
  (|DestroySession PlayerController))

(event Custom|SaveGameCheck
  ;[1 1 1] Check for save game
  (bind _returnvalue (SaveGame|DoesSaveGameExist (Variables|Default|GetPlayerSettingsSave)))
  (if _returnvalue
    (CallFunction|ShowMainMenu)
    (Variables|Default|SetCreatedSaveFile? true)
    (else
      (CallFunction|ShowOptionMenu)
      (Variables|/Script/Engine.PlayerController|SetbShowMouseCursor (Game|GetPlayerController 0) true))))

(event EventHandleNetworkError
  (params (FailureType :type ENetworkFailure%20Enum :default "NetDriverAlreadyExists") (bIsServer :type Boolean))
  ;[1 1 1] Handle Network Error
  (if bIsServer
    _
    (else
      _))
  (Utilities|DisplayErrorMessage (CallFunction|NetErrortoString FailureType)))

(event EventHandleTravelError
  (params (FailureType :type ETravelFailure%20Enum :default "NoLevel"))
  ;[1 1 1] Handle Travel Error
  (Utilities|DisplayErrorMessage (CallFunction|TravelErrortoString FailureType)))

(fn NetErrortoString
  (params (FailureType :type ENetworkFailure%20Enum :default "NetDriverAlreadyExists"))
  (switch Utilities|FlowControl|Switch|SwitchonENetworkFailure FailureType
    (:NetDriverAlreadyExists
      (Variables|Default|SetErrorString "Error : Lost Connection to Host" :!label _label))
    (:NetDriverCreateFailure
      (goto _label))
    (:NetDriverListenFailure
      (goto _label))
    (:ConnectionLost
      (goto _label))
    (:ConnectionTimeout
      (Variables|Default|SetErrorString "Error : Connection Time Out"))
    (:FailureReceived
      (goto _label))
    (:OutdatedClient
      (goto _label))
    (:OutdatedServer
      (goto _label))
    (:PendingConnectionFailure
      (goto _label))
    (:NetGuidMismatch
      (goto _label))
    (:NetChecksumMismatch
      (goto _label)))
  (return (Variables|Default|GetErrorString)))

(fn TravelErrortoString
  (params (FailureType :type ETravelFailure%20Enum :default "NoLevel"))
  (return (Utilities|String|Append "Error : Failed to Travel." (Utilities|String|EnumtoString FailureType))))